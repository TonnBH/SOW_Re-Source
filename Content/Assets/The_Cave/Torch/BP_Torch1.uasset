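; Torch actor with a flickering flare light that turns to face the player camera.
; On BeginPlay, the FlickerLight timeline drives FireFlare intensity as its flicker value scaled by LightIntensity.
; A looping timer calls GetAngle every fifth of a second to yaw the whole actor toward the camera, billboard-style, ignoring height.
; The construction script gives FireFlare a random intensity, which the timeline overrides during play.
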(event `self.ReceiveBeginPlay`
  (`KismetSystemLibrary.K2_SetTimer` null "GetAngle" 0.2 true)
  (bind (_direction _flicker) (`Timeline|FlickerLight`)
    (:`Update`
      (`LightComponent.SetIntensity` (`self.FireFlare`) (* (`self.LightIntensity`) _flicker)))))

(fn `GetAngle`
  (`self.K2_SetActorRotation` (`KismetMathLibrary.Conv_VectorToRotator` (`KismetMathLibrary.Normal` (* (- (`PlayerCameraManager.GetCameraLocation` (`GameplayStatics.GetPlayerCameraManager` 0)) (`self.K2_GetActorLocation`)) (1.0 1.0 0.0))))))

(fn `UserConstructionScript`
  (`LightComponent.SetIntensity` (`self.FireFlare`) (`KismetMathLibrary.RandomFloatInRange` 0.0 10000.0)))